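; VM_OrderModel is a view model that holds a drink order: the selected drink, milk and sugar options, and a text summary.
; Setter functions store each choice.
; SetOrderSummary joins the drink with conditional milk and sugar phrases into OrderSummary, then resets the choices to Coffee with no milk or sugar.
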(fn `SetAddMilk`
  (params (bAddMilk :type Boolean))
  (set `self.bAddMilk` bAddMilk))

(fn `SetAddSugar`
  (params (bAddSugar :type Boolean))
  (set `self.bAddSugar` bAddSugar))

(fn `SetDrink`
  (params (drinkType :type String))
  (set `self.SelectedDrink` drinkType))

(fn `SetOrderSummary`
  (locals (milk :type String) (sugar :type String))
  (if (`self.bAddMilk`)
    (set `local.milk` " with milk "))
  (if (`self.bAddSugar`)
    (if (`self.bAddMilk`)
      (set `local.sugar` " and sugar")
      (else
        (set `local.sugar` " with sugar"))))
  (set `self.OrderSummary` (`KismetTextLibrary.Conv_StringToText` (`KismetStringLibrary.Concat_StrStr` "Your ordered: " (`self.SelectedDrink`) (`local.milk`) (`local.sugar`))))
  (set `self.SelectedDrink` "Coffee")
  (set `self.bAddSugar` false)
  (set `self.bAddMilk` false))